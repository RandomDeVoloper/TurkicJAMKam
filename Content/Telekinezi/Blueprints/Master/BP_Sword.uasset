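; BP_Sword is a throwable sword, apparently for telekinesis, that reports itself and an Enemy reference through GetThrowableActors and toggles a highlight overlay material.
; Tick checks actor speed to switch the saber trail and Swordfly effect on or off.
; Box overlap with a BP_Enemy enables physics simulation on its mesh, with a random one-in-five chance to destroy it.
; The slice and critical-slice sound nodes are disconnected.
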(event `self.ReceiveTick`
  (params (DeltaSeconds :type "Float (single-precision)"))
  (bind _returnvalue (`self.GetVelocity`))
  (bind _ns_sabertrail (`self.NS_SaberTrail`))
  (bind _swordfly (`self.Swordfly`))
  (`PrimitiveComponent.GetPhysicsLinearVelocityAtPoint` (`self.Cube`) _returnvalue "None")
  (if (> (`KismetMathLibrary.VSize` _returnvalue) 200.0)
    (`ActorComponent.SetActive` _ns_sabertrail true false)
    (`GameplayStatics.PlaySoundAtLocation` null (`self.K2_GetActorLocation`) (struct) 1.0 1.0 0.0 null null null null)
    (`ActorComponent.SetActive` _swordfly true false)
    (elif (`ActorComponent.IsActive` _ns_sabertrail)
      (`ActorComponent.Deactivate` _ns_sabertrail)
      (`ActorComponent.SetActive` _swordfly false false))))

(event `self.Box.OnComponentBeginOverlap`
  (params (OverlappedComponent :type "PrimitiveComponent Object Reference") (OtherActor :type "Actor Object Reference") (OtherComp :type "PrimitiveComponent Object Reference") (OtherBodyIndex :type Integer) (bFromSweep :type Boolean) (SweepResult :type "HitResult Structure (by ref)"))
  (bind _asbp_enemy (cast `/Game/Telekinezi/Karakter/BP_Enemy` OtherActor))
  (bind _mesh (`Character.Mesh` _asbp_enemy))
  (`PrimitiveComponent.SetSimulatePhysics` _mesh true)
  (if (== (`KismetMathLibrary.RandomIntegerInRange` 0 4) 0)
    (`/Engine/EditorBlueprintResources/StandardMacros.IsValid` _mesh
      (:`Is Valid`
        (`self.K2_DestroyActor` _asbp_enemy)))))

(event `/Game/Telekinezi/Blueprints/Interfaces/BPI_Interactiable.ChangeMaterial`
  (params (HighLight :type Boolean))
  (bind _cube (`self.Cube`))
  (if HighLight
    (`MeshComponent.SetOverlayMaterial` _cube "/Game/Telekinezi/Materials/HighlightMaterial_Inst.HighlightMaterial_Inst")
    (else
      (`MeshComponent.SetOverlayMaterial` _cube null))))

(fn `GetThrowableActors`
  (returns (Object :type "/Game/Telekinezi/Blueprints/Master/BP_Object Object Reference") (Enemy :type "/Game/Telekinezi/Karakter/BP_Enemy Object Reference"))
  (return self (`self.Enemy`)))

(fn `UserConstructionScript`
  (`parent.UserConstructionScript`)
  (`AddComponent|NODE_AddNiagaraComponent-1`))