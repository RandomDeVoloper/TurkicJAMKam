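; BP_SwordMenu is a sword actor, named as a menu variant, that keeps its saber trail effect (NSSaberTrail) running.
; The construction script turns on auto-activate for the trail, and both BeginPlay and every Tick set it active without a reset.
; Disconnected leftover nodes would deactivate the effect or apply a random trail material and print its name, but never run.
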(event `self.ReceiveBeginPlay`
  (`parent.ReceiveBeginPlay`)
  (`ActorComponent.SetActive` (`self.NS_SaberTrail`) true false :!label _label))

(event `self.ReceiveTick`
  (params (DeltaSeconds :type "Float (single-precision)"))
  (goto _label))

(fn `UserConstructionScript`
  (`parent.UserConstructionScript`)
  (`ActorComponent.SetAutoActivate` (`self.NS_SaberTrail`) true))