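; BP_Sword4 is a sword actor that shows a Niagara saber trail while moving fast.
; Each Tick activates the trail when the actor's speed exceeds a threshold and deactivates it otherwise.
; A physics velocity query on the Cube component also runs each Tick, but the speed check uses only the actor's velocity.
; The construction script adds another Niagara component.
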(event `self.ReceiveTick`
  (params (DeltaSeconds :type "Float (single-precision)"))
  (bind _returnvalue (`self.GetVelocity`))
  (bind _ns_sabertrail (`self.NS_SaberTrail`))
  (`PrimitiveComponent.GetPhysicsLinearVelocityAtPoint` (`self.Cube`) _returnvalue "None")
  (if (> (`KismetMathLibrary.VSize` _returnvalue) 500.0)
    (`ActorComponent.SetActive` _ns_sabertrail true false)
    (elif (`ActorComponent.IsActive` _ns_sabertrail)
      (`ActorComponent.Deactivate` _ns_sabertrail))))

(fn `UserConstructionScript`
  (`parent.UserConstructionScript`)
  (`AddComponent|NODE_AddNiagaraComponent-1`))