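; BPC_HealthSyst is a Blueprint component that tracks a health value for the actor that owns it.
; AddHealth and RemoveHealth raise or lower CurrentHealth by a given amount, clamping it to a fixed 0–100 range.
; The event graph holds no live logic, only disabled default events and an unconnected clamp, and nothing here reacts when health reaches zero.
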(fn `AddHealth`
  (params (Amount :type "Float (double-precision)"))
  (set `self.CurrentHealth` (`KismetMathLibrary.FClamp` (+ (`self.CurrentHealth`) Amount) 0.0 100.0)))

(fn `RemoveHealth`
  (params (Amount :type "Float (double-precision)"))
  (set `self.CurrentHealth` (`KismetMathLibrary.FClamp` (- (`self.CurrentHealth`) Amount) 0.0 100.0)))