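; Day/night controller that alternates 60-second day and night phases, starting with day on BeginPlay.
; DayLoop and NightLoop call each other after delays, triggering StartDay and StartNight.
; Day starts the referenced tent's sound; night stops it and spawns Mongilan enemies at a fixed location, looping over the Days entry at GecenGun, with debug prints.
; GecenGun is never changed in this graph.
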(event `StartDay`
  (`/Game/Developers/USER/Otag/Meshy_AI_Ornate_Yurt_0605235621_texture/StaticMeshes/Otag_BP.StartDayTentSound` (`self.TentRef`) :!label _label))

(event `self.ReceiveBeginPlay`
  (`self.DayLoop`)
  (goto _label))

(event `StartNight`
  (`/Game/Developers/USER/Otag/Meshy_AI_Ornate_Yurt_0605235621_texture/StaticMeshes/Otag_BP.StopDayTentSound` (`self.TentRef`))
  (for _ (`|MakeArray` (`|GetArrayItem` (`self.Days`) (`self.GecenGun`)))
    (`KismetSystemLibrary.PrintString` "Hello")
    (bind _returnvalue (`|SpawnActorFromClass` "/Game/Telekinezi/Karakter/BP_Enemy_Mongilan.BP_Enemy_Mongilan_C" (`KismetMathLibrary.MakeTransform` (10758.0 -3512.75655 -35.579151)) "AdjustIfPossibleButAlwaysSpawn" "MultiplyWithRoot" null null))
    (`KismetSystemLibrary.PrintString` (`KismetSystemLibrary.GetDisplayName` _returnvalue))))

(event `DayLoop`
  (`self.StartDay`)
  (`KismetSystemLibrary.Delay` 60.0)
  (`self.NightLoop`))

(event `NightLoop`
  (`self.StartNight`)
  (`KismetSystemLibrary.Delay` 60.0)
  (`self.DayLoop`))

(fn `UserConstructionScript`)